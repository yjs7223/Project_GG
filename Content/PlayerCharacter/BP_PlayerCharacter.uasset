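; BP_PlayerCharacter is the player character, with a timed dash and configurable jump count and jump velocity.
; IA_Dash calls PlayDash, which resets the timer and picks the horizontal movement direction, or actor forward when nearly still.
; Tick moves the actor by swept location offsets until DashTime elapses, pausing both movement and timer while rising.
; The construction script applies the jump settings, and OnJumped clears horizontal velocity.
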(event `self.ReceiveTick`
  (params (DeltaSeconds :type "Float (single-precision)"))
  (bind (_velocity_x _velocity_y _velocity_z) (`KismetMathLibrary.BreakVector` (`MovementComponent.Velocity` (`self.CharacterMovement`))))
  (`parent.ReceiveTick` DeltaSeconds)
  (if (and (`self.IsDash`) (<= _velocity_z 0.0))
    (set `self.CurrentDashTime` (+ (`self.CurrentDashTime`) DeltaSeconds))
    (`self.K2_SetActorLocation` (+ (`self.K2_GetActorLocation`) (* (`self.DashVelocity`) (* (`self.DashLength`) DeltaSeconds))) true)))

(event `EnhancedInput|/Game/PlayerCharacter/ThirdPerson/Input/Actions/IA_Dash`
  (params (ActionValue :type Boolean) (ElapsedSeconds :type "Float (double-precision)") (TriggeredSeconds :type "Float (double-precision)") (InputAction :type "InputAction Object Reference" :default "/Game/PlayerCharacter/ThirdPerson/Input/Actions/IA_Dash.IA_Dash"))
  (:`Triggered`
    (`self.PlayDash`)))

(event `PlayDash`
  (bind _returnvalue (`KismetMathLibrary.MakeVector` (.x (`MovementComponent.Velocity` (`self.CharacterMovement`))) (.y (`MovementComponent.Velocity` (`self.CharacterMovement`)))))
  (set `self.DashVelocity` (`KismetMathLibrary.Normal` (`KismetMathLibrary.SelectVector` _returnvalue (`self.GetActorForwardVector`) (> (`KismetMathLibrary.VSizeSquared` _returnvalue) 1.0))))
  (set `self.CurrentDashTime` 0.0))

(event `self.OnJumped`
  (bind _charactermovement (`self.CharacterMovement`))
  (bind (_velocity_x _velocity_y _velocity_z) (`KismetMathLibrary.BreakVector` (`MovementComponent.Velocity` _charactermovement)))
  (set `MovementComponent.Velocity` (`KismetMathLibrary.MakeVector` 0.0 0.0 _velocity_z) _charactermovement))

(fn `IsDash`
  (returns (isDash :type Boolean))
  (return (> (`self.DashTime`) (`self.CurrentDashTime`))))

(fn `IsFallingState`
  (returns (isFalling :type Boolean))
  (bind (_velocity_x _velocity_y _velocity_z) (`KismetMathLibrary.BreakVector` (`MovementComponent.Velocity` (`self.CharacterMovement`))))
  (return (< _velocity_z 0.0)))

(fn `UserConstructionScript`
  (`parent.UserConstructionScript`)
  (set `self.JumpMaxCount` (`self.Jumpcount`))
  (set `CharacterMovementComponent.JumpZVelocity` (`self.JumpVelocity`) (`self.CharacterMovement`)))